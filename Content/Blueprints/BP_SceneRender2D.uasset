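; BP_SceneRender2D is an actor, likely a scene capture rig by its name, that glides through the level in repeating passes.
; Each Tick moves it along world -X by a fixed, frame-rate-dependent step and increments a counter.
; When the counter reaches its limit, it resets, and a FlipFlop teleports the actor alternately between two Y-mirrored start positions with mirrored angled rotations.
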(event EventTick
  (params (DeltaSeconds :type Float%20%28single-precision%29))
  (if (< (Variables|Default|GetCounter) 1625)
    (Transformation|AddActorWorldOffset "-2.000000, 0, 0")
    (Math|Integer|IncrementInt (Variables|Default|GetCounter))
    (else
      (Variables|Default|SetCounter 0)
      (Utilities|FlowControl|FlipFlop
        (:A
          (Transformation|SetActorRelativeRotation "-20.000000,110.000000, 0")
          (Transformation|SetActorLocation "-1000.000000,-1500.000000,1000.000000" false false))
        (:B
          (Transformation|SetActorRelativeRotation "-20.000000,-110.000000, 0")
          (Transformation|SetActorLocation "-1000.000000,1500.000000,1000.000000" false false))))))

(fn ConstructionScript)